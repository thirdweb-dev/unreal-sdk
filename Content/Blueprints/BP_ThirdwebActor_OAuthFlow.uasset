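; Sample actor that runs the Thirdweb in-app wallet Google OAuth login flow when play begins.
; BeginPlay creates the wallet handle and checks its connection; if not connected, it starts the default OAuth login and then binds success and failure events.
; An existing connection or successful login leads to printing the wallet address, then disconnecting.
; Errors and OAuth messages are printed on screen.
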(event Custom|OnOAuthSuccess_Event
  (params (WalletHandle :type Integer64) (Message :type String))
  ;[0.04707 0.1143 0.05139] Initiate default OAuth Flow
  ;[0 0 0] Post-Auth with Optional Disconnect Clearing Session
  (Development|PrintString Message)
  (bind (_success _canretry _output) (Class|ThirdwebActor|GetWalletAddress (Variables|Default|GetInAppWalletHandle)))
  (if _success
    (Development|PrintString _output true true "(R=0.112649,G=1.000000,B=0.508361,A=1.000000)" 1e+01)
    (Class|ThirdwebActor|Disconnect (Variables|Default|GetInAppWalletHandle))
    (else
      (Development|PrintString _output true true "(R=1.000000,G=0.000000,B=0.107953,A=1.000000)" 1e+01))))

(event Custom|OnOAuthFailure_Event
  (params (WalletHandle :type Integer64) (Message :type String))
  ;[0.04707 0.1143 0.05139] Initiate default OAuth Flow
  ;[0 0 0] Post-Auth with Optional Disconnect Clearing Session
  (Development|PrintString Message true true "(R=1.000000,G=0.000000,B=0.010696,A=1.000000)"))

(event EventBeginPlay
  ;[0 0 0] Create InAppWallet with OAuth Method
  (bind (_success _canretry _output) (Class|ThirdwebActor|CreateinAppWallet "" "Google"))
  (if _success
    (bind _output_get (Variables|Default|SetInAppWalletHandle (Class|KismetStringLibrary|ToInt64(String) _output)))
    ;[0 0 0] Check if Connected
    (bind (_success_2 _canretry_2 _output_2) (Class|ThirdwebActor|IsConnected _output_get))
    (if _success_2
      (switch string _output_2
        (:true
          ;[0 0 0] Post-Auth with Optional Disconnect Clearing Session
          (bind (_success_3 _canretry_3 _output_3) (Class|ThirdwebActor|GetWalletAddress (Variables|Default|GetInAppWalletHandle)))
          (if _success_3
            (Development|PrintString _output_3 true true "(R=0.112649,G=1.000000,B=0.508361,A=1.000000)" 1e+01)
            (Class|ThirdwebActor|Disconnect (Variables|Default|GetInAppWalletHandle))
            (else
              (Development|PrintString _output_3 true true "(R=1.000000,G=0.000000,B=0.107953,A=1.000000)" 1e+01))))
        (:false
          (Class|ThirdwebActor|LoginwithOauthDefault (Variables|Default|GetInAppWalletHandle))
          ;[0.04707 0.1143 0.05139] Initiate default OAuth Flow
          (EventDispatchers|AssignOnOAuthSuccess (delegate Custom|OnOAuthSuccess_Event))
          (EventDispatchers|AssignOnOAuthFailure (delegate Custom|OnOAuthFailure_Event))))
      (else
        (Development|PrintString _output_2 true true "(R=1.000000,G=0.000000,B=0.126531,A=1.000000)")))
    (else
      (Development|PrintString _output true true "(R=1.000000,G=0.000000,B=0.161514,A=1.000000)" 1e+01))))

(fn ConstructionScript)